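; Base room prefab that sets up a new level room for the victim and poltergeist players when it begins play.
; On BeginPlay it moves the navmesh volume in, spawns a door, sends the victim and up to four poltergeists toward start points, and lerps the camera to the room's view on Tick.
; Invisible walls and ceiling turn blocking when the victim's round starts, and overlapping the victim start notifies the victim of room entry.
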(event `self.ReceiveBeginPlay`
  (bind _returnvalue (`GameplayStatics.GetActorOfClass` "/Game/Blueprints/AI/BP_Victim.BP_Victim_C"))
  (add `Victim.OnRoundStart` _returnvalue (delegate `SolidifyWalls`))
  (`/Game/Blueprints/AI/BP_Victim.RunToNewRoomStart` _returnvalue (`self.VicitmStart`))
  (bind _returnvalue_2 (`GameplayStatics.GetActorOfClass` "/Script/Engine.CameraActor"))
  (bind _output_get (set `self.Camera` _returnvalue_2))
  (set `self.CameraOldPosition` (`self.GetTransform` _output_get))
  (bind _returnvalue_3 (`GameplayStatics.GetActorOfClass` "/Script/NavigationSystem.NavMeshBoundsVolume"))
  (bind _output_get_2 (set `self.Navmesh` _returnvalue_3))
  (`self.K2_SetActorLocation` _output_get_2 (`SceneComponent.K2_GetComponentLocation` (`self.NavmeshSpawn`)) false true)
  (bind _returnvalue_4 (`|SpawnActorFromClass` "/Game/Maps/Prefabs/BP_Door.BP_Door_C" (`SceneComponent.K2_GetComponentToWorld` (`self.DoorSpawnPoint`)) "Undefined" "OverrideRootScale" null null))
  (set `self.Door` _returnvalue_4)
  (bind _outactors (`GameplayStatics.GetAllActorsOfClass` "/Script/Poltergeists.PlayerPoltergeist"))
  (for (_array_element _array_index) _outactors
    (switch `int` _array_index
      (:`0`
        (set `PlayerPoltergeist.RunToLocation` (`SceneComponent.K2_GetComponentLocation` (`self.PlayerStart1`)) _array_element))
      (:`1`
        (set `PlayerPoltergeist.RunToLocation` (`SceneComponent.K2_GetComponentLocation` (`self.PlayerStart2`)) _array_element))
      (:`2`
        (set `PlayerPoltergeist.RunToLocation` (`SceneComponent.K2_GetComponentLocation` (`self.PlayerStart3`)) _array_element))
      (:`3`
        (set `PlayerPoltergeist.RunToLocation` (`SceneComponent.K2_GetComponentLocation` (`self.PlayerStart4`)) _array_element)))))

(event `SolidifyWalls`
  (`PrimitiveComponent.SetCollisionProfileName` (`self.InvisibleWall1`) "BlockAll")
  (`PrimitiveComponent.SetCollisionProfileName` (`self.InvisibleWall2`) "BlockAll")
  (`PrimitiveComponent.SetCollisionProfileName` (`self.InvisibleCeiling`) "BlockAll"))

(event `self.VicitmStart.OnComponentBeginOverlap`
  (params (OverlappedComponent :type "PrimitiveComponent Object Reference") (OtherActor :type "Actor Object Reference") (OtherComp :type "PrimitiveComponent Object Reference") (OtherBodyIndex :type Integer) (bFromSweep :type Boolean) (SweepResult :type "HitResult Structure (by ref)"))
  (bind _asvictim (cast `Victim` OtherActor))
  (`Victim.ReceiveEnterNewRoom` _asvictim))

(event `self.ReceiveTick`
  (params (DeltaSeconds :type "Float (single-precision)"))
  (if (not (`self.CameraArrived`))
    (bind _output_get (set `self.CameraLerpAmount` (`KismetMathLibrary.FClamp` (+ (/ DeltaSeconds 1.5) (`self.CameraLerpAmount`)))))
    (`self.K2_SetActorTransform` (`self.Camera`) (`KismetMathLibrary.TLerp` (`self.CameraOldPosition`) (`SceneComponent.K2_GetComponentToWorld` (`self.CameraStart`)) _output_get) false false)
    (if (== _output_get 1.0)
      (set `self.CameraArrived` true))))

(fn `UserConstructionScript`)