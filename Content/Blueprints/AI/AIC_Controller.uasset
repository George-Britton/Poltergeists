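; AI controller that can send its pawn to randomly chosen scare spots in the level.
; On BeginPlay it caches every actor tagged "Scare" in ScareSpots.
; GetRandomScareSpot picks one of them at random, and GoToRandomScareSpot walks the pawn there with SimpleMoveToActor.
; The controller does not start movement itself, as nothing in its own graphs calls GoToRandomScareSpot.
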(event `self.ReceiveBeginPlay`
  (bind _outactors (`GameplayStatics.GetAllActorsWithTag` "Scare"))
  (set `self.ScareSpots` _outactors))

(fn `GetRandomScareSpot`
  (returns (ScareSpot :type "Actor Object Reference"))
  (bind _scarespots (`self.ScareSpots`))
  (return (`|GetArrayItem` _scarespots (`KismetMathLibrary.RandomIntegerInRange` 0 (- (`KismetArrayLibrary.Array_Length` _scarespots) 1)))))

(fn `GoToRandomScareSpot`
  (`AIBlueprintHelperLibrary.SimpleMoveToActor` self (`self.GetRandomScareSpot`)))

(fn `UserConstructionScript`)