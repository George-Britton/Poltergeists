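; BP_Victim is the AI-moved victim character that roams a room's scare spots and flees through a door.
; During a round it loops AIMoveTo between random ScareSpots, pausing for less time as Fear rises, until RoundOver.
; RunAway heads for the Door and opens it, and RunToNewRoomStart moves to StartLocation and signals room entry, both retrying on failure.
; Snare and Unsnare divide and restore walk speed by the trap's TrapStrength.
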(event `self.RoundStart`
  ;[1 1 1] Sends the victim running around the room
  (`KismetSystemLibrary.Delay` 0.5)
  (bind _returnvalue (`self.GetRandomScareSpot` :!label _label))
  (`/Engine/EditorBlueprintResources/StandardMacros.IsValid` _returnvalue
    (:`Is Valid`
      (`|AIMoveTo` self (`self.K2_GetActorLocation` _returnvalue) null 50.0
        (:`OnSuccess`
          _)
        (:`OnFail`
          _))
      (`KismetSystemLibrary.Delay` (/ (- 200.0 (`self.Fear`)) 100.0))
      (if (not (`self.RoundOver`))
        (goto _label)))
    (:`Is Not Valid`
      (`self.GetScareSpots`)
      (goto _label))))

(event `self.RunAway`
  ;[1 1 1] Run away demo
  (bind _returnvalue (`GameplayStatics.GetActorOfClass` "/Script/Poltergeists.Door"))
  (bind _output_get (set `self.Door` _returnvalue))
  (`/Engine/EditorBlueprintResources/StandardMacros.IsValid` _output_get
    (:`Is Valid`
      (`|AIMoveTo` self (0.0 0.0 0.0) _returnvalue 100.0 true :!label _label_2
        (:`OnSuccess`
          (`Door.ReceiveOpen` _returnvalue))
        (:`OnFail`
          (`KismetSystemLibrary.Delay` 0.2)
          (goto _label_2))))))

(event `self.Snare`
  (params (Trap :type "Trap Object Reference"))
  (bind _charactermovement (`self.CharacterMovement`))
  ;[1 1 1] Caught in trap stuff
  (set `CharacterMovementComponent.MaxWalkSpeed` (/ (`CharacterMovementComponent.MaxWalkSpeed` _charactermovement) (`Trap.TrapStrength` Trap)) _charactermovement))

(event `self.Unsnare`
  (params (Trap :type "Trap Object Reference"))
  (bind _charactermovement (`self.CharacterMovement`))
  ;[1 1 1] Caught in trap stuff
  (set `CharacterMovementComponent.MaxWalkSpeed` (* (`CharacterMovementComponent.MaxWalkSpeed` _charactermovement) (`Trap.TrapStrength` Trap)) _charactermovement))

(event `RunToNewRoomStart`
  (`|AIMoveTo` self (`self.StartLocation`) null 50.0 true :!label _label_3
    (:`OnSuccess`
      (`KismetSystemLibrary.Delay` 0.5)
      (`self.ReceiveEnterNewRoom`))
    (:`OnFail`
      (`KismetSystemLibrary.Delay` 0.2)
      (goto _label_3))))

(fn `GetScareSpots`
  (bind _outactors (`GameplayStatics.GetAllActorsOfClass` "/Script/Poltergeists.ScareSpot"))
  (set `self.ScareSpots` _outactors)
  (return))

(fn `UserConstructionScript`)