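; Player poltergeist Blueprint that can trigger a scare ability and carry an item.
; Activating a scare creates a cooldown counter widget, passes it the cooldown and a reference to the poltergeist, and adds it to the viewport.
; Each tick while an item is held, the physics handle target moves to a set distance in front of the actor.
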(event `self.ActivateScare`
  (bind _returnvalue (`|CreateWidget` "/Game/Blueprints/Widgets/CooldownCounter.CooldownCounter_C"))
  (set `/Game/Blueprints/Widgets/CooldownCounter.Cooldown` (`self.Cooldown`) _returnvalue)
  (set `/Game/Blueprints/Widgets/CooldownCounter.Poltergeist` self _returnvalue)
  (`UserWidget.AddToViewport` _returnvalue 0))

(event `self.ReceiveTick`
  (params (DeltaSeconds :type "Float (single-precision)"))
  (if (`self.IsItemHeld`)
    (`PhysicsHandleComponent.SetTargetLocation` (`self.PhysicsHandle`) (+ (`self.K2_GetActorLocation`) (* (`self.GetActorForwardVector`) (`self.ItemHeldDistance`))))))

(fn `UserConstructionScript`)