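; SS_Television is a television scare spot that changes its screen material as it is triggered and finishes.
; Activation applies the telly screen material and removes any existing recharge timer widget.
; When the scare finishes, it switches the screen to M_Vertex and adds a RechargeTimer widget to the viewport, passing it the recharge time and a reference to itself.
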(event `self.ActivateScareSpot`
  (bind _rechargewidget (`self.RechargeWidget`))
  (`PrimitiveComponent.SetMaterial` (`self.Screen`) 0 "/Game/Geometry/Meshes/LivingRoom/M_TellyScreen.M_TellyScreen")
  (`/Engine/EditorBlueprintResources/StandardMacros.IsValid` _rechargewidget
    (:`Is Valid`
      (`Widget.RemoveFromParent` _rechargewidget))))

(event `self.OnScareFinish`
  (`PrimitiveComponent.SetMaterial` (`self.Screen`) 0 "/Game/Geometry/Meshes/LivingRoom/M_Vertex.M_Vertex")
  (bind _returnvalue (`|CreateWidget` "/Game/Blueprints/Widgets/RechargeTimer.RechargeTimer_C"))
  (set `/Game/Blueprints/Widgets/RechargeTimer.Recharge` (`self.RechargeTime`) _returnvalue)
  (set `/Game/Blueprints/Widgets/RechargeTimer.ParentScareSpot` self _returnvalue)
  (bind _output_get (set `self.RechargeWidget` _returnvalue))
  (`UserWidget.AddToViewport` _output_get 0))

(fn `UserConstructionScript`)