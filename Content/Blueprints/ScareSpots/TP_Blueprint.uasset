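; TP_Blueprint is an actor whose particle effect responds to how far it moves.
; Each Tick it compares its location with the previous frame's and takes the distance as Speed, without dividing by delta time.
; It feeds Speed into the particle system's TPSpawnRate instance parameter, so the effect can follow the motion.
; The zero-speed branch does nothing, as the Activate and Deactivate calls are left unconnected.
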(event `self.ReceiveBeginPlay`
  (set `self.ThisFrameLoc` (`self.K2_GetActorLocation`)))

(event `self.ReceiveTick`
  (params (DeltaSeconds :type "Float (single-precision)"))
  (bind _output_get (set `self.LastFrameLoc` (`self.ThisFrameLoc`)))
  (bind _output_get_2 (set `self.ThisFrameLoc` (`self.K2_GetActorLocation`)))
  (bind _output_get_3 (set `self.Speed` (`KismetMathLibrary.VSize` (- _output_get_2 _output_get))))
  (set `ParticleSystemComponent.InstanceParameters` (`|MakeArray` (make `ParticleSysParam` "TPSpawnRate" "PSPT_Scalar" _output_get_3) :!type "ParticleSysParam Structure") (`self.ParticleSystem1`))
  (if (== _output_get_3 0.0)
    _))

(fn `UserConstructionScript`)