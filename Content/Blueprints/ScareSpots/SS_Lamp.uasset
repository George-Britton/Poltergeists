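; SS_Lamp is a scare spot Blueprint for a lamp that animates its lighting when activated.
; ActivateScareSpot plays a timeline whose alpha directly drives the intensity of the top and bottom spotlights.
; OnScareFinish creates a CooldownCounter widget, passes it this spot and its cooldown time, and adds it to the viewport.
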(event `self.ActivateScareSpot`
  (bind (_direction _alpha) (`Timeline|Timeline_0`)
    (:`Update`
      (`LightComponent.SetIntensity` (`self.Spotlight_Top`) _alpha)
      (`LightComponent.SetIntensity` (`self.SpotLight_Bottom`) _alpha))))

(event `self.OnScareFinish`
  (bind _returnvalue (`|CreateWidget` "/Game/Blueprints/Widgets/CooldownCounter.CooldownCounter_C"))
  (set `/Game/Blueprints/Widgets/CooldownCounter.ParentScareSpot` self _returnvalue)
  (set `/Game/Blueprints/Widgets/CooldownCounter.Cooldown` (`self.CooldownTime`) _returnvalue)
  (`UserWidget.AddToViewport` _returnvalue 0))

(fn `UserConstructionScript`)