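; BP_Cupboard_Door_Oven is a kitchen oven scare spot that bursts into flames when activated.
; On activation, a timeline rotates the scare spot mesh about its roll axis to open the door, unless it is already open.
; The flame effect and sound start once the door is open.
; When the scare finishes, both stop, while the door rotation is left as is.
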(event `self.ActivateScareSpot`
  (if (`self.Open`)
    (`ActorComponent.Activate` (`self.Flames`) false :!label _label)
    (`AudioComponent.Play` (`self.FlameSounds`) 0.0)
    (else
      (bind (_direction _alpha) (`Timeline|Timeline_0`)
        (:`Update`
          (`SceneComponent.K2_SetRelativeRotation` (`self.ScareSpotMeshComponent`) (`KismetMathLibrary.MakeRotator` _alpha) false false))
        (:`Finished`
          (goto _label))))))

(event `self.OnScareFinish`
  (`ActorComponent.Deactivate` (`self.Flames`))
  (`AudioComponent.Stop` (`self.FlameSounds`)))

(fn `UserConstructionScript`)