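; Toilet roll prop that shrinks while its Yate flag is set, until it runs out.
; Each tick first updates the paper particle system from the Yate, empty and active states, then reduces the roll mesh's X/Y world scale by delta time times ShrinkSpeed, keeping Z.
; At a minimum scale it marks the roll empty and stops the particles.
; The construction script clamps ShrinkSpeed.
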(event `self.ReceiveTick`
  (params (DeltaSeconds :type "Float (single-precision)"))
  (`|ExecutionSequence`
    (:`then_0`
      (`self.(De)Activate Particles`))
    (:`then_1`
      (`self.ShrinkRoll` DeltaSeconds))))

(fn `UserConstructionScript`
  (set `self.ShrinkSpeed` (`KismetMathLibrary.FClamp` (`self.ShrinkSpeed`))))